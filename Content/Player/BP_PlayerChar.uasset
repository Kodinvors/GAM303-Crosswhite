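; BP_PlayerChar is the player character, handling movement, look, jump, object interaction, score and health.
; Interact line-traces from the camera and sends an interface message to the hit actor, or drops the stored object while IsHolding, which is never set true here.
; Toss drops the held object and pushes a BP_PhysicsPickup along the camera's forward vector.
; Score and health changes print to screen, and health falling below zero quits the game.
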(event Custom|AddScore
  (params (Add%20Amount :type Integer))
  ;[0 0 0] AddScore
  (bind _output_get (Variables|Default|SetScore (+ (Variables|Default|GetScore) Add%20Amount)))
  (Development|PrintString (Utilities|String|ToString(Integer) _output_get)))

(event Input|EnhancedActionEvents|EnhancedInputActionInput_Movement
  (params (ActionValue :type Vector%202D%20Structure) (ElapsedSeconds :type Float%20%28double-precision%29) (TriggeredSeconds :type Float%20%28double-precision%29) (InputAction :type Input%20Action%20Object%20Reference :default "/Game/Inputs/Input_Movement.Input_Movement"))
  (bind _returnvalue (Pawn|GetControlRotation :!class /Script/Engine.Pawn))
  ;[0 0 0] Player Movement
  (Pawn|Input|AddMovementInput (Math|Vector|GetRightVector (Math|Rotator|MakeRotator (.roll _returnvalue) 0.0 (.yaw _returnvalue))) (.x ActionValue) false)
  (Pawn|Input|AddMovementInput (Math|Vector|GetForwardVector (Math|Rotator|MakeRotator 0.0 0.0 (.yaw _returnvalue))) (.y ActionValue) false))

(event Input|EnhancedActionEvents|EnhancedInputActionInput_Look
  (params (ActionValue :type Vector%202D%20Structure) (ElapsedSeconds :type Float%20%28double-precision%29) (TriggeredSeconds :type Float%20%28double-precision%29) (InputAction :type Input%20Action%20Object%20Reference :default "/Game/Inputs/Input_Look.Input_Look"))
  ;[0 0 0] Player Movement
  (Pawn|Input|AddControllerYawInput (.x ActionValue))
  (Pawn|Input|AddControllerPitchInput (.y ActionValue)))

(event Input|EnhancedActionEvents|EnhancedInputActionInput_Jump
  (params (ActionValue :type Boolean) (ElapsedSeconds :type Float%20%28double-precision%29) (TriggeredSeconds :type Float%20%28double-precision%29) (InputAction :type Input%20Action%20Object%20Reference :default "/Game/Inputs/Input_Jump.Input_Jump"))
  ;[0 0 0] Player Movement
  (:Started
    (Character|Jump))
  (:Canceled
    (Character|StopJumping)))

(event Input|EnhancedActionEvents|EnhancedInputActionInput_Interact
  (params (ActionValue :type Boolean) (ElapsedSeconds :type Float%20%28double-precision%29) (TriggeredSeconds :type Float%20%28double-precision%29) (InputAction :type Input%20Action%20Object%20Reference :default "/Game/Inputs/Input_Interact.Input_Interact"))
  (bind _camera (Variables|Default|GetCamera))
  (bind _returnvalue (Transformation|GetWorldLocation _camera))
  ;[0 0 0] Input_Interact
  (:Started
    (if (Variables|Default|GetisHolding?)
      (Class|InterfaceInteract|INTDrop(Message) (Variables|Default|GetHitObject))
      (Variables|Default|SetisHolding? false)
      (else
        (bind (_outhit _returnvalue_2) (Collision|LineTraceByChannel _returnvalue (+ _returnvalue (* (Math|Vector|GetForwardVector _camera) 8e+02)) "TraceTypeQuery1" false 0 "ForDuration"))
        (if _returnvalue_2
          (Variables|Default|SetHitObject (.HitActor (Collision|BreakHitResult _outhit)))
          (Class|InterfaceInteract|INTInteract(Message) (.HitActor (Collision|BreakHitResult _outhit)) self))))))

(event EventBeginPlay)

(event Game|Damage|EventAnyDamage
  (params (Damage :type Float%20%28single-precision%29) (DamageType :type Damage%20Type%20Object%20Reference) (InstigatedBy :type Controller%20Object%20Reference) (DamageCauser :type Actor%20Object%20Reference))
  ;[0 0 0] AnyDamage
  (bind _output_get (Variables|Default|SetHealth (- (Variables|Default|GetHealth) Damage)))
  (Development|PrintString (Utilities|String|ToString(Float) _output_get))
  (if (< (Variables|Default|GetHealth) 0.0)
    (Game|QuitGame 0 "Quit" false)))

(event Input|ActionEvents|InputActionToss
  (params (Key :type Key%20Structure :default "None"))
  (bind _hitobject (Variables|Default|GetHitObject))
  ;[0 0 0] Toss
  (:Pressed
    (if (Variables|Default|GetisHolding?)
      (Class|InterfaceInteract|INTDrop(Message) _hitobject)
      (Variables|Default|SetisHolding? false)
      (bind _asbp_physics_pickup (Utilities|Casting|CastToBP_PhysicsPickup _hitobject))
      (Physics|AddForce (Variables|/Game/Interactables/BP_PhysicsPickup.BP_PhysicsPickup_C|GetCube _asbp_physics_pickup) (* (Math|Vector|GetForwardVector (Variables|Default|GetCamera)) (Variables|Default|GetThrowForce)) "None" true))))

(fn ConstructionScript)